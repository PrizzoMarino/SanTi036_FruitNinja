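; BP_Fruit is a fruit actor that can be flagged as sliced and appears intended for a slicing game.
; Its construction script picks a random mesh from FruitMesh and copies it from the static mesh component into a procedural mesh with collision.
; Three seconds after BeginPlay, it destroys itself unless IsSliced is set.
; The slicing itself is not handled in these graphs.
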(event `self.ReceiveBeginPlay`
  (`KismetSystemLibrary.Delay` 3.0)
  (if (not (`self.isSliced`))
    (`self.K2_DestroyActor`)))

(fn `UserConstructionScript`
  (bind _fruit (`self.Fruit`))
  (`StaticMeshComponent.SetStaticMesh` _fruit (`|GetArrayItem` (`self.FruitMesh`) (`KismetMathLibrary.RandomIntegerInRange` 0 (- (`KismetArrayLibrary.Array_Length` (`self.FruitMesh`)) 1))))
  (`KismetProceduralMeshLibrary.CopyProceduralMeshFromStaticMeshComponent` _fruit 0 (`self.ProceduralMesh`) true))