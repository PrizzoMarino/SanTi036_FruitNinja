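; Grabbable VR sword that slices procedural meshes its Plane component overlaps.
; On grab it enables input and messages the motion controller's owner to hide the left hand, avoiding a hard pawn reference.
; A DoOnce, reset on end overlap, cuts along the plane with a capped other half, which gets physics and a radial impulse.
; Unconnected leftover logic covers trace-based BP_Fruit slicing and a swing-speed check.
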(event `self.ReceiveBeginPlay`)

(event `self.ReceiveTick`
  (params (DeltaSeconds :type "Float (single-precision)")))

(event `self.GrabComponent.OnGrabbed`
  (`self.EnableInput` (`GameplayStatics.GetPlayerController` 0))
  (message `/Game/VRTemplate/Blueprints/BPI_PawnAnim.HideUnhideHand` (`ActorComponent.GetOwner` (`/Game/VRTemplate/Blueprints/GrabComponent.MotionControllerRef` (`self.GrabComponent`))) true false))

(event `self.Plane.OnComponentBeginOverlap`
  (params (OverlappedComponent :type "PrimitiveComponent Object Reference") (OtherActor :type "Actor Object Reference") (OtherComp :type "PrimitiveComponent Object Reference") (OtherBodyIndex :type Integer) (bFromSweep :type Boolean) (SweepResult :type "HitResult Structure (by ref)"))
  (bind _plane (`self.Plane`))
  (bind _returnvalue (`SceneComponent.K2_GetComponentLocation` _plane))
  (`/Engine/EditorBlueprintResources/StandardMacros.DoOnce` false :!label _label
    (:`Completed`
      (bind _asprocedural_mesh_component (cast `ProceduralMeshComponent` OtherComp))
      (`KismetSystemLibrary.PrintString` "sliced")
      (bind _outotherhalfprocmesh (`KismetProceduralMeshLibrary.SliceProceduralMesh` _asprocedural_mesh_component _returnvalue (`SceneComponent.GetUpVector` _plane) true "CreateNewSectionForCap"))
      (`PrimitiveComponent.SetSimulatePhysics` _outotherhalfprocmesh true)
      (`PrimitiveComponent.AddRadialImpulse` _outotherhalfprocmesh _returnvalue 50.0 100.0 "RIF_Constant" false))))

(event `self.Plane.OnComponentEndOverlap`
  (params (OverlappedComponent :type "PrimitiveComponent Object Reference") (OtherActor :type "Actor Object Reference") (OtherComp :type "PrimitiveComponent Object Reference") (OtherBodyIndex :type Integer))
  (goto _label :!via `Reset`))

(fn `UserConstructionScript`)