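; BP_FruitSpawner is an actor that continuously spawns BP_Fruit actors around its own location.
; A looping timer started on BeginPlay fires SpawnFruit, which prints a debug message and spawns a fruit at a randomized horizontal and slightly raised offset.
; Each new fruit's Fruit component then receives a radial impulse from a fixed world-space origin, not one relative to the spawner or fruit.
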(event `self.ReceiveBeginPlay`
  (`KismetSystemLibrary.K2_SetTimerDelegate` (delegate `Spawn Fruit`) 1.2 true))

(event `Spawn Fruit`
  (bind _returnvalue (`KismetMathLibrary.RandomFloatInRange` -200.0 200.0))
  (`KismetSystemLibrary.PrintString` "Spawn")
  (bind _returnvalue_2 (`|SpawnActorFromClass` "/Game/Blueprints/BP_Fruit.BP_Fruit_C" (`KismetMathLibrary.MakeTransform` (`KismetMathLibrary.MakeVector` (+ (.x (`self.K2_GetActorLocation`)) _returnvalue) (+ (.y (`self.K2_GetActorLocation`)) _returnvalue) (+ (.z (`self.K2_GetActorLocation`)) (`KismetMathLibrary.RandomFloatInRange` 0.0 50.0)))) "Undefined" "MultiplyWithRoot" null null))
  (`PrimitiveComponent.AddRadialImpulse` (`/Game/Blueprints/BP_Fruit.Fruit` _returnvalue_2) (0.0 0.0 50.0) 50.0 100.0 "RIF_Constant" false))

(fn `UserConstructionScript`)