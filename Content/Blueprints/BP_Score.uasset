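; BP_Score is an actor that displays a score and a countdown, and opens the Demo level when time runs out.
; BeginPlay shows the zero-padded score on a text render and starts a looping one-second timer.
; Each tick of that timer decrements and redraws the countdown, loading Demo at zero.
; The AddScore event increments and redraws the score, but without the zero-padding used at start.
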(event `AddScore`
  (bind _output_get (set `self.Score` (+ (`self.Score`) 1)))
  (`TextRenderComponent.K2_SetText` (`self.TextRender`) (`KismetTextLibrary.Conv_IntToText` _output_get false false 4)))

(event `self.ReceiveBeginPlay`
  (`TextRenderComponent.K2_SetText` (`self.TextRender`) (`KismetTextLibrary.Conv_IntToText` (`self.Score`) false false 4))
  (`KismetSystemLibrary.K2_SetTimerDelegate` (delegate `TimeGo`) 1.0 true))

(event `TimeGo`
  (bind _output_get (set `self.Timerr` (- (`self.Timerr`) 1)))
  (`TextRenderComponent.K2_SetText` (`self.Timer`) (`KismetTextLibrary.Conv_IntToText` _output_get false false 2))
  (if (== (`self.Timerr`) 0)
    (`GameplayStatics.OpenLevelBySoftObjectPtr` "/Game/Jongmyo/Map/Demo.Demo")))

(fn `UserConstructionScript`)